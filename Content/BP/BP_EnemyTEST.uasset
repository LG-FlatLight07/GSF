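; BP_EnemyTEST is a test enemy that periodically fires lasers at the player.
; A countdown timer starts at a random one to four seconds, ticks down each frame, then resets to a fixed interval after every shot.
; Each shot spawns a BP_Laser at the enemy, aims it at the player pawn, launches it, and turns the enemy to face the player.
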(event `self.ReceiveBeginPlay`
  (set `self.timer` (`KismetMathLibrary.RandomFloatInRange` 1.0 4.0)))

(event `self.ReceiveTick`
  (params (DeltaSeconds :type "Float (single-precision)"))
  (bind _laseractor (`self.LaserActor`))
  (`|ExecutionSequence`
    (:`then_0`
      ;[1 1 1] excute per 3 seconds
      (bind _output_get (set `self.timer` (- (`self.timer`) DeltaSeconds)))
      (if (< _output_get 0.0)
        (set `self.timer` 3.0)
        ;[1 1 1] spawn laser and launch
        (bind _returnvalue (`|SpawnActorFromClass` "/Game/BP/BP_Laser.BP_Laser_C" (`self.GetTransform`) "AlwaysSpawn" "MultiplyWithRoot" null null))
        (bind _output_get_2 (set `self.LaserActor` _returnvalue))
        (`/Engine/EditorBlueprintResources/StandardMacros.IsValid` _output_get_2
          (:`Is Valid`
            (`self.K2_SetActorRotation` _laseractor (`KismetMathLibrary.FindLookAtRotation` (`self.K2_GetActorLocation`) (`self.K2_GetActorLocation` (`GameplayStatics.GetPlayerPawn` 0))) false)
            (`/Game/BP/BP_Laser.LaunchLaser` _laseractor (`self.K2_GetActorLocation`))
            ;[1 1 1] rotate enemy
            (`self.K2_SetActorRotation` (`KismetMathLibrary.FindLookAtRotation` (`self.K2_GetActorLocation`) (`self.K2_GetActorLocation` (`GameplayStatics.GetPlayerPawn` 0))))))))))

(fn `UserConstructionScript`)