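; Beam projectile that damages BPI_Enemy actors, passing a guard-break value, and destroys itself on hit, ignoring its launcher.
; It spawns with a random local offset and is destroyed once its age exceeds a limit.
; Each Tick, Chase steps it toward a valid Target by Speed, unscaled by delta time.
; Lazer mode takes its location from Lazar, whose straight LaunchVec step appears unconnected.
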(event `self.ReceiveBeginPlay`
  (bind _randomrange (`self.randomRange`))
  (bind _returnvalue (* _randomrange -1.0))
  (`self.K2_AddActorLocalTransform` (`KismetMathLibrary.MakeTransform` (`KismetMathLibrary.MakeVector` (`KismetMathLibrary.RandomFloatInRange` _returnvalue _randomrange) (`KismetMathLibrary.RandomFloatInRange` _returnvalue _randomrange) (`KismetMathLibrary.RandomFloatInRange` _returnvalue _randomrange)))))

(event `self.ReceiveTick`
  (params (DeltaSeconds :type "Float (single-precision)"))
  (`|ExecutionSequence`
    (:`then_0`
      (switch `/Game/_Main/Enemy/E_BeaMode` (`self.mode`)
        (:`NewEnumerator0`
          (`self.K2_SetActorLocation` (`self.Lazar`)))
        (:`NewEnumerator1`
          (bind _returnvalue (`self.Chase`)
            (:`は有効である`
              (`self.K2_SetActorLocation` _returnvalue))))))
    (:`then_1`
      (`self.AgeCount` DeltaSeconds))))

(event `self.Sphere.OnComponentBeginOverlap`
  (params (OverlappedComponent :type "PrimitiveComponent Object Reference") (OtherActor :type "Actor Object Reference") (OtherComp :type "PrimitiveComponent Object Reference") (OtherBodyIndex :type Integer) (bFromSweep :type Boolean) (SweepResult :type "HitResult Structure (by ref)"))
  (if (!= OtherActor (`self.Launcher`))
    (bind _asbpi_enemy (cast `/Game/_Main/Enemy/BPI_Enemy` OtherActor))
    (`/Game/_Main/Enemy/BPI_Enemy.Damage` _asbpi_enemy (`self.damage`) (`self.guardBreak`))
    (`self.K2_DestroyActor`)))

(fn `UserConstructionScript`)