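; Enemy actor with health and guard gauges that registers with BP_GSFGameMode and sets up lock-on and beam components.
; Damage lowers HP and guard, then updates the auto, manual and concentration lock-on widgets.
; Depleted guard triggers a one-time break, after which HP damage is scaled by a bias.
; At zero HP it unregisters from the game mode and destroys itself.
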(event `self.ReceiveBeginPlay`
  (`/Game/_Main/Enemy/BPC_LockOn.Set` (`self.BPC_LockOn`) (`self.LockOnWidget`) (`self.ManualLockOnWidget`) (`self.ConccentrationLockOnWidget`) self)
  (set `/Game/_Main/Enemy/BPC_Beam.Beam` (`self.Beam`) (`self.BPC_Beam`))
  (`/Game/_Main/Enemy/BPC_Beam.Set` (`self.BPC_Beam`) self)
  (bind _asbp_gsfgame_mode (cast `/Game/_Main/BP_GSFGameMode` (`GameplayStatics.GetGameMode`)))
  (`/Game/_Main/BP_GSFGameMode.AddEnemy` _asbp_gsfgame_mode self)
  (set `self.HP` (`self.MaxHP`))
  (set `self.GuardPower` (`self.MaxGuard`))
  (`self.UpdateHealthGage`))

(event `/Game/_Main/Enemy/BPI_Enemy.Damage`
  (params (Damage :type "Float (double-precision)") (GuardBreak :type "Float (double-precision)"))
  (if (`self.break`)
    (set `self.HP` (`KismetMathLibrary.FClamp` (- (`self.HP`) (* Damage (`self.breakDamageBias`))) 0.0 (`self.MaxHP`)))
    (else
      (set `self.HP` (`KismetMathLibrary.FClamp` (- (`self.HP`) Damage) 0.0 (`self.MaxHP`)))))
  (set `self.GuardPower` (`KismetMathLibrary.FClamp` (- (`self.GuardPower`) GuardBreak) 0.0 (`self.MaxGuard`)))
  (`self.UpdateHealthGage`)
  (if (<= (`self.HP`) 0.0)
    (bind _asbp_gsfgame_mode (cast `/Game/_Main/BP_GSFGameMode` (`GameplayStatics.GetGameMode`)))
    (`/Game/_Main/BP_GSFGameMode.RemoveEnemy` _asbp_gsfgame_mode self)
    (`self.K2_DestroyActor`)
    (elif (<= (`self.GuardPower`) 0.0)
      (`/Engine/EditorBlueprintResources/StandardMacros.DoOnce` false
        (:`Completed`
          (`self.GuardBreak`))))))

(event `/Game/_Main/Enemy/BPI_Enemy.LookOn`
  (params (lookOn :type Boolean)))

(event `GuardBreak`
  (set `self.break` true))

(fn `UserConstructionScript`)