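; Enemy component that decides whether its enemy is lock-on targetable and shows the matching indicator widget, using references passed in through Set.
; Every Tick it branches on player input: concentration hides both indicators, manual aim shows one, and auto aim the other.
; Both aim modes require recent rendering, player proximity and a Visibility trace hit toward the player to set the enemy's LockOn.
; Manual aim also requires the enemy's screen position to be near the aim cursor.
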(event `self.ReceiveTick`
  (params (DeltaSeconds :type "Float (single-precision)"))
  (bind _enemy (`self.Enemy`))
  (bind _enemy_2 (`self.Enemy`))
  (bind _returnvalue (`Actor.K2_GetActorLocation` _enemy_2))
  (bind _returnvalue_2 (`Actor.K2_GetActorLocation` _enemy))
  (bind _asbp_gsfcharacter (cast `/Game/_Main/Character/BP_GSFCharacter` (`GameplayStatics.GetPlayerPawn` 0)))
  (bind _returnvalue_3 (`GSFCharacter.InputComp` _asbp_gsfcharacter))
  (if (`GSFInputComp.bPressedConcentrationKey` _returnvalue_3)
    ;[0 0.2969 0.06773] 集中
    (`SceneComponent.SetVisibility` (`self.Widget`) false false)
    (`SceneComponent.SetVisibility` (`self.ManualWidget`) false false)
    (elif (`GSFInputComp.bPressedManualAimKey` _returnvalue_3)
      ;[0 0.4993 1] マニュアルエイム
      (`SceneComponent.SetVisibility` (`self.Widget`) false false)
      (if (`Actor.WasRecentlyRendered` (`self.Enemy`) 0.1)
        (if (< (`KismetMathLibrary.Vector_Distance` (`Actor.K2_GetActorLocation` (`self.Enemy`)) (`Actor.K2_GetActorLocation` (`GameplayStatics.GetPlayerPawn` 0))) (`self.ManualAimDis`))
          (bind _asbp_gsfcharacter_2 (cast `/Game/_Main/Character/BP_GSFCharacter` (`GameplayStatics.GetPlayerPawn` 0)))
          (if (< (`KismetMathLibrary.Distance2D` (`GameplayStatics.ProjectWorldToScreen` (`GameplayStatics.GetPlayerController` 0) _returnvalue) (`/Game/_Main/Widget/LockOn/WBP_ManualAim.moveInput` (`/Game/_Main/Character/BP_GSFCharacter.ManualAimWidget` _asbp_gsfcharacter_2))) (`self.ManualAimRange`))
            (bind (_outhit _returnvalue_4) (`KismetSystemLibrary.LineTraceSingle` _returnvalue (`Actor.K2_GetActorLocation` (`GameplayStatics.GetPlayerPawn` 0)) "TraceTypeQuery1" false (`|MakeArray` _enemy_2 :!type "Actor Object Reference")))
            (if _returnvalue_4
              (bind _manualwidget (`self.ManualWidget`)
                (:`then`
                  (`SceneComponent.SetVisibility` _manualwidget true false)
                  (set `/Game/_Main/Enemy/BP_enemy.LockOn` true (`self.Enemy`)))
                (:`else`))
              (else
                (bind _manualwidget_2 (`self.ManualWidget` :!label _label)
                  (:`then`
                    (`SceneComponent.SetVisibility` _manualwidget_2 false false)
                    (set `/Game/_Main/Enemy/BP_enemy.LockOn` false (`self.Enemy`)))
                  (:`else`))))
            (else
              (goto _label)))
          (else
            (goto _label)))
        (else
          (goto _label)))
      (else
        ;[1 0 0.08214] オートエイム
        (`SceneComponent.SetVisibility` (`self.ManualWidget`) false false)
        (if (`Actor.WasRecentlyRendered` (`self.Enemy`) 0.1)
          (if (< (`KismetMathLibrary.Vector_Distance` _returnvalue_2 (`Actor.K2_GetActorLocation` (`GameplayStatics.GetPlayerPawn` 0))) (`self.AutoAimDis`))
            (bind (_outhit_2 _returnvalue_5) (`KismetSystemLibrary.LineTraceSingle` _returnvalue_2 (`Actor.K2_GetActorLocation` (`GameplayStatics.GetPlayerPawn` 0)) "TraceTypeQuery1" false (`|MakeArray` _enemy :!type "Actor Object Reference")))
            (if _returnvalue_5
              (bind _widget (`self.Widget`)
                (:`then`
                  (`SceneComponent.SetVisibility` _widget true false)
                  (set `/Game/_Main/Enemy/BP_enemy.LockOn` true (`self.Enemy`)))
                (:`else`))
              (else
                (bind _widget_2 (`self.Widget` :!label _label_2)
                  (:`then`
                    (`SceneComponent.SetVisibility` _widget_2 false false)
                    (set `/Game/_Main/Enemy/BP_enemy.LockOn` false (`self.Enemy`)))
                  (:`else`))))
            (else
              (goto _label_2)))
          (else
            (goto _label_2)))))))

(event `Set`
  (params (widget :type "WidgetComponent Object Reference") (ManualWidget :type "WidgetComponent Object Reference") (ConcentrationWidget :type "WidgetComponent Object Reference") (enemy :type "/Game/_Main/Enemy/BP_enemy Object Reference"))
  (set `self.Widget` widget)
  (set `self.ManualWidget` ManualWidget)
  (set `self.ConcentrationWidget` ConcentrationWidget)
  (set `self.Enemy` enemy))