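; BPC_Beam is an enemy component that periodically fires Beam actors at the player.
; It receives its Enemy reference through Set and counts a timer down on Tick, pausing while that enemy is in its Break state.
; A randomized first delay varies the opening shot, then each BeamCycle spawns a Beam at the owner, launched toward the player pawn with configured speed, lifetime and mode.
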(event `self.ReceiveTick`
  (params (DeltaSeconds :type "Float (single-precision)"))
  (bind _returnvalue (`GameplayStatics.GetPlayerPawn` 0))
  (bind _returnvalue_2 (`Actor.K2_GetActorLocation` (`self.GetOwner`)))
  (bind _enemy (`self.enemy`)
    (:`then`
      (if (not (`/Game/_Main/Enemy/BP_enemy.break` _enemy))
        (bind _output_get (set `self.Timer` (- (`self.Timer`) DeltaSeconds)))
        (if (< _output_get 0.0)
          (set `self.Timer` (`self.beamCycle`))
          (`|SpawnActorFromClass` (`self.Beam`) (`KismetMathLibrary.Conv_VectorToTransform` _returnvalue_2) "Undefined" "OverrideRootScale" null (`KismetMathLibrary.Normal` (- (`Actor.K2_GetActorLocation` _returnvalue) _returnvalue_2)) (`self.beamSpeed`) (`self.BeamAgeLimit`) (`self.Mode`) _returnvalue (`self.enemy`) null))))
    (:`else`)))

(event `self.ReceiveBeginPlay`
  (set `self.Timer` (`KismetMathLibrary.RandomFloatInRange` 1.0 4.0)))

(event `Set`
  (params (ebnemy :type "/Game/_Main/Enemy/BP_enemy Object Reference"))
  (set `self.enemy` ebnemy))