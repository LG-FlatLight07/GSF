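; Player character Blueprint that adds homing beam fire, concentration lock-on and manual aiming to its parent character, plus air jump and dash montages.
; Tick fires gated beam volleys at random locked-on enemies, denser during concentration, and locks the enemy nearest center while concentrating, using game mode queries.
; Concentration attack wire-moves to that enemy, which non-beam hitbox overlaps cancel.
; Camera input moves the manual-aim reticle within screen margins.
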(event `self.ReceiveBeginPlay`
  (bind _returnvalue (`|CreateWidget` "/Game/_Main/Widget/WBP_ManualAim.WBP_ManualAim_C"))
  (bind _output_get (set `self.ManualAimWidget` _returnvalue))
  (`UserWidget.AddToViewport` _output_get 0)
  (`Widget.SetVisibility` _output_get "Hidden")
  (bind _returnvalue_2 (`|CreateWidget` "/Game/_Main/Widget/WBP_Concentration.WBP_Concentration_C"))
  (bind _output_get_2 (set `self.ConcentraionWidget` _returnvalue_2))
  (`UserWidget.AddToViewport` _output_get_2 0)
  (`Widget.SetVisibility` _output_get_2 "Hidden"))

(event `self.AirDash`
  (`parent.AirDash`)
  (if (not (`GSFInputComp.bPressedManualAimKey` (`self.inputComp`)))
    (`|PlayMontage` (`self.mesh`) "/Game/_Main/Character/Anim/Dodge_Montage.Dodge_Montage")))

(event `self.AirJump`
  (`parent.AirJump`)
  (if (not (`GSFInputComp.bPressedManualAimKey` (`self.inputComp`)))
    (`|PlayMontage` (`self.mesh`) "/Game/_Main/Character/Anim/Jump_Montage.Jump_Montage")))

(event `self.ManualAim`
  (params (look :type Boolean))
  (bind (_returnvalue_x _returnvalue_y) (`KismetMathLibrary.BreakVector2D` (`WidgetLayoutLibrary.GetViewportSize`)))
  (`parent.ManualAim` look)
  (if look
    (set `Widget.Visibility` "Visible" (`self.ManualAimWidget`))
    (else
      (set `Widget.Visibility` "Hidden" (`self.ManualAimWidget`))))
  (set `/Game/_Main/Widget/WBP_ManualAim.moveInput` (`KismetMathLibrary.MakeVector2D` (/ _returnvalue_x 2.0) (/ _returnvalue_y 2.0)) (`self.ManualAimWidget`)))

(event `self.ReceiveTick`
  (params (DeltaSeconds :type "Float (single-precision)"))
  (bind (_returnvalue_x _returnvalue_y) (`KismetMathLibrary.BreakVector2D` (`WidgetLayoutLibrary.GetViewportSize`)))
  (bind _concentraionwidget (`self.ConcentraionWidget`))
  (bind _manualaimwidget (`self.ManualAimWidget`))
  (bind _manualaimwidget_2 (`self.ManualAimWidget`))
  (bind _moveinput_x (`KismetMathLibrary.BreakVector2D` (`/Game/_Main/Widget/WBP_ManualAim.moveInput` _manualaimwidget_2)))
  (bind (_moveinput_x_2 _moveinput_y) (`KismetMathLibrary.BreakVector2D` (`/Game/_Main/Widget/WBP_ManualAim.moveInput` _manualaimwidget)))
  (`parent.ReceiveTick` 0.0)
  (`|ExecutionSequence`
    (:`then_0`
      (if (`GSFInputComp.bPressedConcentrationKey` (`self.inputComp`))
        (if (`GSFInputComp.bPresseBulletKey` (`self.inputComp`))
          (`/Engine/EditorBlueprintResources/StandardMacros.DoOnce` false :!label _label
            (:`Completed`
              (for _ (range (+ (* (`self.MaxBeamLaunchNum`) 3) 1))
                (bind _asbp_gsfgame_mode (cast `/Game/_Main/BP_GSFGameMode` (`GameplayStatics.GetGameMode`)))
                (bind _output (`/Game/_Main/BP_GSFGameMode.GetRandomLockOnEnemy` _asbp_gsfgame_mode))
                (if (`KismetSystemLibrary.IsValid` _output)
                  (`self.Shot` _output)
                  (`self.Shot` _output)
                  (`self.Shot` _output)
                  (`self.Shot` _output)
                  (`self.Shot` _output)
                  (`self.Shot` _output)))
              (`KismetSystemLibrary.Delay` 0.027)
              (goto _label :!via `Reset`))))
        (elif (`GSFInputComp.bPresseBulletKey` (`self.inputComp`))
          (`/Engine/EditorBlueprintResources/StandardMacros.DoOnce` false :!label _label_2
            (:`Completed`
              (for _ (range (+ (`self.MaxBeamLaunchNum`) 1))
                (bind _asbp_gsfgame_mode_2 (cast `/Game/_Main/BP_GSFGameMode` (`GameplayStatics.GetGameMode`)))
                (bind _output_2 (`/Game/_Main/BP_GSFGameMode.GetRandomLockOnEnemy` _asbp_gsfgame_mode_2))
                (if (`KismetSystemLibrary.IsValid` _output_2)
                  (`|SpawnActorFromClass` "/Game/_Main/Beam/BP_Beam_Player.BP_Beam_Player_C" (`KismetMathLibrary.Conv_VectorToTransform` (`self.RandomLaunchPoint`)) "Undefined" "OverrideRootScale" null (0.0 0.0 0.0) (`self.BeamSpeed`) (`self.BeamAge`) "NewEnumerator1" _output_2 self null)
                  (`KismetSystemLibrary.Delay` 0.01)))
              (`KismetSystemLibrary.Delay` 0.07)
              (goto _label_2 :!via `Reset`))))))
    (:`then_1`
      (if (`GSFInputComp.bPressedConcentrationKey` (`self.inputComp`))
        (`Widget.SetVisibility` _concentraionwidget "Visible")
        (bind _asbp_gsfgame_mode_3 (cast `/Game/_Main/BP_GSFGameMode` (`GameplayStatics.GetGameMode`)))
        (bind _nearcanteractor1 (`/Game/_Main/BP_GSFGameMode.GetNearCenterEnemy` _asbp_gsfgame_mode_3))
        (if (`KismetSystemLibrary.IsValid` _nearcanteractor1)
          (bind _output_get (set `self.ConcentrationEnemy` _nearcanteractor1))
          (`/Game/_Main/BP_GSFGameMode.ConcentrationLockOn` _asbp_gsfgame_mode_3 _output_get))
        (else
          (`Widget.SetVisibility` _concentraionwidget "Hidden")
          (bind _asbp_gsfgame_mode_4 (cast `/Game/_Main/BP_GSFGameMode` (`GameplayStatics.GetGameMode`)))
          (`/Game/_Main/BP_GSFGameMode.DisableConcentrationLockOn` _asbp_gsfgame_mode_4))))
    (:`then_2`
      (bind _asbp_gsfgame_mode_5 (cast `/Game/_Main/BP_GSFGameMode` (`GameplayStatics.GetGameMode`)))
      (bind (_x _y) (`KismetMathLibrary.BreakVector2D` (`GSFCamera.inputValue` (`GSFGameMode.camera` _asbp_gsfgame_mode_5))))
      (bind (_x_2 _y_2) (`KismetMathLibrary.BreakVector2D` (+ (* (`KismetMathLibrary.MakeVector2D` _x (* _y -1.0)) (`self.ManualAimSensitivity`)) (`/Game/_Main/Widget/WBP_ManualAim.moveInput` (`self.ManualAimWidget`)))))
      (if (> _x_2 (* _returnvalue_x 0.95))
        _
        (elif (not (< _x_2 (* _returnvalue_x 0.05)))
          (set `/Game/_Main/Widget/WBP_ManualAim.moveInput` (`KismetMathLibrary.MakeVector2D` _x_2 _moveinput_y) _manualaimwidget)))
      (if (> _y_2 (* _returnvalue_y 0.9))
        _
        (elif (not (< _y_2 (* _returnvalue_y 0.1)))
          (set `/Game/_Main/Widget/WBP_ManualAim.moveInput` (`KismetMathLibrary.MakeVector2D` _moveinput_x _y_2) _manualaimwidget_2))))))

(event `self.Attack`
  (`parent.Attack`)
  (`KismetSystemLibrary.PrintString` "attack"))

(event `self.ConcentrationAttack`
  (bind _concentrationenemy (`self.ConcentrationEnemy`))
  (`parent.ConcentrationAttack`)
  (`KismetSystemLibrary.PrintString` "concentAttack")
  (if (`GSFInputComp.bPressedConcentrationKey` (`self.inputComp`))
    (`/Engine/EditorBlueprintResources/StandardMacros.IsValid` _concentrationenemy
      (:`Is Valid`
        (`GSFMoveComp.WireMove` (`self.moveComp`) (`self.K2_GetActorLocation` _concentrationenemy) 0.0)
        (bind _asbp_gsfgame_mode (cast `/Game/_Main/BP_GSFGameMode` (`GameplayStatics.GetGameMode`)))
        (bind _near1 (`/Game/_Main/BP_GSFGameMode.GetNearPlayerEnemy` _asbp_gsfgame_mode))
        (`/Engine/EditorBlueprintResources/StandardMacros.IsValid` _near1
          (:`Is Valid`
            (if (not (== _near1 _concentrationenemy))
              (`PrimitiveComponent.SetCollisionEnabled` (`self.hitBox`) "NoCollision")
              (`KismetSystemLibrary.Delay` 0.15)
              (`PrimitiveComponent.SetCollisionEnabled` (`self.hitBox`) "QueryAndPhysics"))))))))

(event `self.ConcentrationBeam`
  (`parent.ConcentrationBeam`))

(event `self.hitBox.OnComponentBeginOverlap`
  (params (OverlappedComponent :type "PrimitiveComponent Object Reference") (OtherActor :type "Actor Object Reference") (OtherComp :type "PrimitiveComponent Object Reference") (OtherBodyIndex :type Integer) (bFromSweep :type Boolean) (SweepResult :type "HitResult Structure (by ref)"))
  (bind _movecomp (`self.moveComp`))
  (if (`GSFMoveComp.bWire` _movecomp)
    (if (!= (`GameplayStatics.GetObjectClass` OtherActor) "/Game/_Main/Beam/BP_Beam.BP_Beam_C")
      (set `GSFMoveComp.bWire` false _movecomp))))

(fn `UserConstructionScript`)